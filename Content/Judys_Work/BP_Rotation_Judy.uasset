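; BP_Rotation_Judy is an actor that spins its root component a full turn around the roll axis.
; On BeginPlay it starts a timeline whose looping and play rate come from the Looping and TimeToComplete variables.
; Each timeline update lerps the track value into a 0 to 360 degree relative roll on DefaultSceneRoot.
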(event Custom|StartRotateAnimation
  (bind _movement (Variables|Default|GetMovement))
  (Components|Timeline|SetLooping _movement (Variables|Default|GetLooping))
  (Components|Timeline|SetPlayRate _movement (/ 1.0 (Variables|Default|GetTimeToComplete)))
  (bind _newtrack_0 (Timeline|Movement PlayFromStart)
    (:Update
      (Transformation|SetRelativeRotation (Variables|Default|GetDefaultSceneRoot) (Math|Rotator|MakeRotator (Math|Float|Lerp 0.0 3.6e+02 _newtrack_0) 0.0 0.0) false false))))

(event EventBeginPlay
  (CallFunction|StartRotateAnimation))

(fn ConstructionScript)