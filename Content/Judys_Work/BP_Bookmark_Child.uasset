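; BP_Bookmark_Child is a child Blueprint that tilts itself to the surface normal found by a line trace at BeginPlay.
; The Visibility trace ends below the root along its down vector, but its start omits the root's location, unlike the drawn debug line.
; The hit normal and root forward vector build the new rotation via MakeRotFromXZ, without checking for a hit.
; Debug prints and drawings show the result.
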(event EventBeginPlay
  (bind _defaultsceneroot (Variables|Default|GetDefaultSceneRoot))
  (bind _returnvalue (Transformation|GetWorldLocation _defaultsceneroot))
  (bind _returnvalue_2 (Math|Vector|GetUpVector _defaultsceneroot))
  (bind _returnvalue_3 (* _returnvalue_2 -4e+02))
  (bind _returnvalue_4 (+ _returnvalue _returnvalue_3))
  (|CallParentFunction)
  (bind _outhit (Collision|LineTraceByChannel (* _returnvalue_2 -1e+02) _returnvalue_4 "TraceTypeQuery1" false 0 "None"))
  (Rendering|Debug|DrawDebugLine _returnvalue _returnvalue_4 "(R=1.000000,G=0.000000,B=0.035615,A=1.000000)" 1e+01 3.0)
  (Development|PrintString (Utilities|String|ToString(Vector) (.ImpactPoint (Collision|BreakHitResult _outhit))))
  (Development|PrintString (Utilities|GetDisplayName (.HitActor (Collision|BreakHitResult _outhit))))
  (Rendering|Debug|DrawDebugPoint (.ImpactPoint (Collision|BreakHitResult _outhit)) 1e+02 "(R=1.000000,G=0.000000,B=0.958208,A=1.000000)" 1e+01)
  (Transformation|SetActorRotation (Math|Rotator|MakeRotfromXZ (Math|Vector|GetForwardVector _defaultsceneroot) (.Normal (Collision|BreakHitResult _outhit)))))

(event Collision|EventActorBeginOverlap
  (params (OtherActor :type Actor%20Object%20Reference))
  (|CallParentFunction OtherActor) ; This node is disabled and will not be called.\nDrag off pins to build functionality.
)

(event EventTick
  (params (DeltaSeconds :type Float%20%28single-precision%29))
  (|CallParentFunction DeltaSeconds) ; This node is disabled and will not be called.\nDrag off pins to build functionality.
)

(fn ConstructionScript
  (|CallParentFunction))