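; Spline path mover that carries the player pawn and/or an optional root actor along its spline, optionally auto-starting after a short delay.
; A looping or oscillating timeline, rate-scaled by TimeToComplete, feeds MoveObjects, which converts alpha to spline distance and teleports both.
; With RotatePlayer, the pawn takes spline rotation but only spline height, keeping its X/Y.
; When the non-oscillating timeline finishes, it opens LevelName.
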(event Custom|StartMoveAnimation
  (bind _oscillatingmovement (Variables|Default|GetOscillatingMovement))
  (bind _movement (Variables|Default|GetMovement))
  (if (Variables|Default|GetOscillating)
    (Components|Timeline|SetLooping _oscillatingmovement true)
    (Components|Timeline|SetPlayRate _oscillatingmovement (/ 1.0 (Variables|Default|GetTimeToComplete)))
    (bind _newtrack_0 (Timeline|OscillatingMovement Play)
      (:Update
        (CallFunction|MoveObjects _newtrack_0)))
    (else
      (Components|Timeline|SetLooping _movement (Variables|Default|GetLooping))
      (Components|Timeline|SetPlayRate _movement (/ 1.0 (Variables|Default|GetTimeToComplete)))
      (bind _move (Timeline|Movement Play)
        (:Update
          (CallFunction|MoveObjects _move))
        (:Finished
          (Game|OpenLevel(byName) (Variables|Default|GetLevelName)))))))

(event Custom|MoveObjects
  (params (Alpha :type Float%20%28single-precision%29))
  (bind _returnvalue (Game|Player|GetPlayerPawn 0))
  (bind _spline (Variables|Default|GetSpline))
  (bind _movableobjectroot (Variables|Default|GetMovableObjectRoot))
  (bind _returnvalue_2 (Spline|GetSplineLength _spline))
  (bind _returnvalue_3 (Transformation|GetActorLocation _returnvalue))
  (bind (_x _y) (Math|Vector|BreakVector _returnvalue_3))
  (bind _returnvalue_4 (Math|Float|Lerp 0.0 _returnvalue_2 Alpha))
  (bind _returnvalue_5 (Spline|GetLocationatDistanceAlongSpline _spline _returnvalue_4 "World"))
  (bind _returnvalue_6 (Spline|GetRotationatDistanceAlongSpline _spline _returnvalue_4 "World"))
  (Utilities|FlowControl|Sequence
    (:then_0
      (if (Variables|Default|GetMovePlayer)
        (if (Variables|Default|GetRotatePlayer)
          (Transformation|SetActorLocationAndRotation _returnvalue (Math|Vector|MakeVector _x _y (.Z (Math|Vector|BreakVector _returnvalue_5))) _returnvalue_6 false true)
          (else
            (Transformation|SetActorLocation _returnvalue _returnvalue_5 false true)))))
    (:then_1
      (if (Utilities|IsValid _movableobjectroot)
        (Transformation|SetActorLocationAndRotation _movableobjectroot _returnvalue_5 _returnvalue_6 false true)))))

(event EventBeginPlay
  (if (Variables|Default|GetPlayOnStart)
    (Utilities|FlowControl|Delay 5.0)
    (CallFunction|StartMoveAnimation)))

(fn ConstructionScript)