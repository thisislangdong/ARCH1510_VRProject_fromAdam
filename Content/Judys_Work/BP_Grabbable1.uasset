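; VR grabbable actor that, when released from a hand, destroys itself and reveals its linked DiagramPiece.
; BeginPlay places that piece at an offset from the pawn's left hand, attaches and hides it.
; CollisionBox overlaps with tagged hand components arm left or right grabbing.
; Tick polls the VRPawn's grip states to attach the object to the gripping hand, allowing hand-to-hand transfer, and detach it on release.
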(event OnComponentBeginOverlap(CollisionBox)
  (params (OverlappedComponent :type Primitive%20Component%20Object%20Reference) (OtherActor :type Actor%20Object%20Reference) (OtherComp :type Primitive%20Component%20Object%20Reference) (OtherBodyIndex :type Integer) (bFromSweep :type Boolean) (SweepResult :type Hit%20Result%20Structure%20%28by%20ref%29))
  (if (Components|ComponentHasTag OtherComp "Hand")
    (Variables|Default|SetCollidedHand OtherComp)
    (Variables|Default|SetPrepareForGrabbing true)
    (if (Components|ComponentHasTag OtherComp "LeftHand")
      (Variables|Default|SetPreparedForLeft true)
      (Variables|Default|SetLeftHand OtherComp)
      (else
        (Variables|Default|SetPreparedForRight true)
        (Variables|Default|SetRightHand OtherComp)))))

(event OnComponentEndOverlap(CollisionBox)
  (params (OverlappedComponent :type Primitive%20Component%20Object%20Reference) (OtherActor :type Actor%20Object%20Reference) (OtherComp :type Primitive%20Component%20Object%20Reference) (OtherBodyIndex :type Integer))
  (if (Components|ComponentHasTag OtherComp "Hand")
    (Variables|Default|SetPrepareForGrabbing false)
    (if (Components|ComponentHasTag OtherComp "LeftHand")
      (Variables|Default|SetPreparedForLeft false)
      (else
        (Variables|Default|SetPreparedForRight false)))))

(event Custom|AttachToParent
  (Rendering|SetActorHiddenInGame (Variables|Default|GetDiagramPiece) false)
  (Actor|DestroyActor))

(event EventTick
  (params (DeltaSeconds :type Float%20%28single-precision%29))
  (Utilities|FlowControl|Sequence
    (:then_0
      (if (Variables|Default|GetPreparedForLeft)
        (if (Variables|Default|GetGrabbedByLeft)
          (if (not (Variables|/Game/VRTemplate/Blueprints/VRPawn.VRPawn_C|GetIsLeftGrip (Variables|Default|GetPlayerPawn)))
            (Transformation|DetachFromComponent (Variables|Default|GetDefaultSceneRoot) "KeepWorld" "KeepWorld" "KeepWorld" true)
            (Variables|Default|SetGrabbedByLeft false)
            (CallFunction|AttachtoParent))
          (elif (Variables|/Game/VRTemplate/Blueprints/VRPawn.VRPawn_C|GetIsLeftGrip (Variables|Default|GetPlayerPawn))
            (Transformation|AttachComponentToComponent (Variables|Default|GetLeftHand) "None" "KeepWorld" "KeepWorld" "KeepWorld" true)
            (Variables|Default|SetGrabbedByLeft true)
            (Variables|Default|SetGrabbedByRight false)))))
    (:then_1
      (if (Variables|Default|GetPreparedForRight)
        (if (Variables|Default|GetGrabbedByRight)
          (if (not (Variables|/Game/VRTemplate/Blueprints/VRPawn.VRPawn_C|GetIsRightGrip (Variables|Default|GetPlayerPawn)))
            (Transformation|DetachFromComponent (Variables|Default|GetDefaultSceneRoot) "KeepWorld" "KeepWorld" "KeepWorld" true)
            (Variables|Default|SetGrabbedByRight false)
            (CallFunction|AttachtoParent))
          (elif (Variables|/Game/VRTemplate/Blueprints/VRPawn.VRPawn_C|GetIsRightGrip (Variables|Default|GetPlayerPawn))
            (Transformation|AttachComponentToComponent (Variables|Default|GetRightHand) "None" "KeepWorld" "KeepWorld" "KeepWorld" true)
            (Variables|Default|SetGrabbedByRight true)
            (Variables|Default|SetGrabbedByLeft false)))))))

(event EventBeginPlay
  (bind _diagrampiece (Variables|Default|GetDiagramPiece))
  (bind _rootcomponent (Variables|/Script/Engine.Actor|GetRootComponent _diagrampiece))
  (bind _asvrpawn (Utilities|Casting|CastToVRPawn (Game|Player|GetPlayerPawn 0)))
  (Variables|Default|SetPlayerPawn _asvrpawn)
  (Transformation|SetWorldLocation _rootcomponent (+ (Transformation|GetWorldLocation (Variables|/Game/VRTemplate/Blueprints/VRPawn.VRPawn_C|GetLeftHand _asvrpawn)) (Variables|Default|GetLocationOffset)) false true)
  (Transformation|SetWorldRotation _rootcomponent (Transformation|GetWorldRotation (Variables|/Game/VRTemplate/Blueprints/VRPawn.VRPawn_C|GetLeftHand _asvrpawn)) false false)
  (Transformation|AttachComponentToComponent _diagrampiece 0 "None" "KeepWorld" "KeepWorld" "KeepWorld" true)
  (Rendering|SetActorHiddenInGame (Variables|Default|GetDiagramPiece) true))

(fn ConstructionScript)