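; BP_Trigger is a VR interaction trigger that fires when a hand is inside its collision box and that hand's trigger is pressed.
; Overlaps with Hand-tagged components arm the left or right side, using the LeftHand tag to tell them apart.
; Tick polls the VRPawn's trigger states and calls the empty CustomTriggerEvent, latched by JustClicked until both triggers are released.
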(event OnComponentBeginOverlap(CollisionBox)
  (params (OverlappedComponent :type Primitive%20Component%20Object%20Reference) (OtherActor :type Actor%20Object%20Reference) (OtherComp :type Primitive%20Component%20Object%20Reference) (OtherBodyIndex :type Integer) (bFromSweep :type Boolean) (SweepResult :type Hit%20Result%20Structure%20%28by%20ref%29))
  (if (Components|ComponentHasTag OtherComp "Hand")
    (if (Components|ComponentHasTag OtherComp "LeftHand")
      (Variables|Default|SetPreparedForLeft true)
      (else
        (Variables|Default|SetPreparedForRight true)))))

(event OnComponentEndOverlap(CollisionBox)
  (params (OverlappedComponent :type Primitive%20Component%20Object%20Reference) (OtherActor :type Actor%20Object%20Reference) (OtherComp :type Primitive%20Component%20Object%20Reference) (OtherBodyIndex :type Integer))
  (if (Components|ComponentHasTag OtherComp "Hand")
    (if (Components|ComponentHasTag OtherComp "LeftHand")
      (Variables|Default|SetPreparedForLeft false)
      (else
        (Variables|Default|SetPreparedForRight false)))))

(event Custom|CustomTriggerEvent)

(event EventTick
  (params (DeltaSeconds :type Float%20%28single-precision%29))
  (bind _playerpawn (Variables|Default|GetPlayerPawn))
  (Utilities|FlowControl|Sequence
    (:then_0
      (if (Variables|Default|GetPreparedForLeft)
        (if (Variables|/Game/VRTemplate/Blueprints/VRPawn.VRPawn_C|GetIsLeftTrigger (Variables|Default|GetPlayerPawn))
          (if (not (Variables|Default|GetJustClicked)) :!label _label
            (CallFunction|CustomTriggerEvent)
            (Variables|Default|SetJustClicked true)))))
    (:then_1
      (if (Variables|Default|GetPreparedForRight)
        (if (Variables|/Game/VRTemplate/Blueprints/VRPawn.VRPawn_C|GetIsRightTrigger (Variables|Default|GetPlayerPawn))
          (goto _label))))
    (:then_2
      (if (not (or (Variables|/Game/VRTemplate/Blueprints/VRPawn.VRPawn_C|GetIsLeftTrigger _playerpawn) (Variables|/Game/VRTemplate/Blueprints/VRPawn.VRPawn_C|GetIsRightTrigger _playerpawn)))
        (Variables|Default|SetJustClicked false)))))

(event EventBeginPlay
  (bind _asvrpawn (Utilities|Casting|CastToVRPawn (Game|Player|GetPlayerPawn 0)))
  (Variables|Default|SetPlayerPawn _asvrpawn))

(fn ConstructionScript)