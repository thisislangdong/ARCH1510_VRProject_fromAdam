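; BP_CollideAndTeleport is an interaction actor that teleports the player pawn when a component tagged "Head" enters its collision box.
; CollisionBox overlap calls TeleportToTarget, which moves player pawn 0 to the world location and rotation of the TeleportTarget component.
; On BeginPlay it hides the Capsule and Arrow components, leaving their children's visibility untouched.
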(event OnComponentBeginOverlap(CollisionBox)
  (params (OverlappedComponent :type Primitive%20Component%20Object%20Reference) (OtherActor :type Actor%20Object%20Reference) (OtherComp :type Primitive%20Component%20Object%20Reference) (OtherBodyIndex :type Integer) (bFromSweep :type Boolean) (SweepResult :type Hit%20Result%20Structure%20%28by%20ref%29))
  (if (Components|ComponentHasTag OtherComp "Head")
    (CallFunction|TeleporttoTarget)))

(event EventBeginPlay
  (Rendering|SetVisibility (Variables|Default|GetCapsule) false false))

(event Collision|EventActorBeginOverlap
  (params (OtherActor :type Actor%20Object%20Reference)))

(event EventTick
  (params (DeltaSeconds :type Float%20%28single-precision%29)))

(fn ConstructionScript)

(fn TeleporttoTarget
  (bind _teleporttarget (Variables|Default|GetTeleportTarget))
  (Transformation|Teleport (Game|Player|GetPlayerPawn 0) (Transformation|GetWorldLocation _teleporttarget) (Transformation|GetWorldRotation _teleporttarget)))