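; Puzzle trigger that repositions target pieces according to the arrangement of grabbable pieces, using the first piece of each set as reference.
; CustomTriggerEvent computes the relative transform between the first and each other grabbable piece.
; TransformTarget teleports the matching target piece onto the first target, then adds that offset as a world-space delta.
; ScaleTransform can rescale offsets by the target-to-grabbable scale ratio but is never called here.
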(event EventBeginPlay
  (|CallParentFunction) ; This node is disabled and will not be called.\nDrag off pins to build functionality.
)

(event Collision|EventActorBeginOverlap
  (params (OtherActor :type Actor%20Object%20Reference)))

(event EventTick
  (params (DeltaSeconds :type Float%20%28single-precision%29))
  (|CallParentFunction DeltaSeconds) ; This node is disabled and will not be called.\nDrag off pins to build functionality.
)

(event EventCustomTriggerEvent
  (for (_ _array_index) (Variables|Default|GetTargetPieces)
    (if (> _array_index 0)
      (bind _returnvalue (CallFunction|GetRelativeTransform _array_index))
      (CallFunction|TransformTarget _returnvalue _array_index))))

(fn ConstructionScript
  (|CallParentFunction))

(fn GetRelativeTransform
  (params (Index :type Integer))
  (return (Class|KismetMathLibrary|ConvertTransformtoRelative (Transformation|GetActorTransform (Utilities|Array|Get(acopy) (Variables|Default|GetGrabbablePieces))) (Transformation|GetActorTransform (Utilities|Array|Get(acopy) (Variables|Default|GetGrabbablePieces) Index)))))

(fn ScaleTransform
  (params (Transform :type Transform))
  (bind (_location _rotation _scale) (Math|Transform|BreakTransform Transform))
  (return (Math|Transform|MakeTransform (* _location (/ (Variables|Default|GetTargetScale) (Variables|Default|GetGrabbableScale))) _rotation _scale)))

(fn TransformTarget
  (params (Transform :type Transform) (Index :type Integer))
  (bind _targetpieces (Variables|Default|GetTargetPieces))
  (bind _targetpieces_2 (Variables|Default|GetTargetPieces))
  (bind _output (Utilities|Array|Get(acopy) _targetpieces))
  (bind _output_2 (Utilities|Array|Get(acopy) _targetpieces_2 Index))
  (bind _returnvalue (Transformation|GetActorTransform _output))
  (Transformation|SetActorLocationAndRotation _output_2 (.location _returnvalue) (.rotation _returnvalue) false true)
  (Class|Actor|AddActorWorldTransform _output_2 (Math|Transform|MakeTransform (.location Transform) (.rotation Transform) "1,1,1") false false))