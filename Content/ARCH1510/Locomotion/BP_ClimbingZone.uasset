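; BP_ClimbingZone is a box volume that switches the VR player's locomotion mode while their hands are inside, presumably for climbing.
; Shortly after BeginPlay it caches the VRPawn and its current Locomotion as the default.
; Overlaps from components tagged "Hand" increment or decrement a counter.
; Any hand entering applies the zone's mode, and the default returns only when the count drops to zero.
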(event OnComponentBeginOverlap(Box)
  (params (OverlappedComponent :type Primitive%20Component%20Object%20Reference) (OtherActor :type Actor%20Object%20Reference) (OtherComp :type Primitive%20Component%20Object%20Reference) (OtherBodyIndex :type Integer) (bFromSweep :type Boolean) (SweepResult :type Hit%20Result%20Structure%20%28by%20ref%29))
  (if (Components|ComponentHasTag OtherComp "Hand")
    (bind _result (Math|Integer|IncrementInt (Variables|Default|GetNumber%20Overlapped))
      (:%20%20
        (Variables|Default|SetNumber%20Overlapped _result)
        (Variables|/Game/VRTemplate/Blueprints/VRPawn.VRPawn_C|SetLocomotion (Variables|Default|GetVRPlayer) "NewEnumerator2")))))

(event OnComponentEndOverlap(Box)
  (params (OverlappedComponent :type Primitive%20Component%20Object%20Reference) (OtherActor :type Actor%20Object%20Reference) (OtherComp :type Primitive%20Component%20Object%20Reference) (OtherBodyIndex :type Integer))
  (if (Components|ComponentHasTag OtherComp "Hand")
    (bind _result (Math|Integer|DecrementInt (Variables|Default|GetNumber%20Overlapped))
      (:%20%20
        (bind _output_get (Variables|Default|SetNumber%20Overlapped _result))
        (if (== _output_get 0)
          (Variables|/Game/VRTemplate/Blueprints/VRPawn.VRPawn_C|SetLocomotion (Variables|Default|GetVRPlayer) (Variables|Default|GetDefaultLocomotion)))))))

(event EventBeginPlay
  (Utilities|FlowControl|Delay 0.2)
  (bind _asvrpawn (Utilities|Casting|CastToVRPawn (Game|Player|GetPlayerPawn 0)))
  (bind _output_get (Variables|Default|SetVRPlayer _asvrpawn))
  (Variables|Default|SetDefaultLocomotion (Variables|/Game/VRTemplate/Blueprints/VRPawn.VRPawn_C|GetLocomotion _output_get)))

(fn ConstructionScript)