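; VR locomotion controller that attaches to the pawn's right hand and steps through location bookmarks, displaying the current name.
; MoveNext and MovePrevious either teleport the pawn or, with ChangeGravity, rotate and shift WorldModelRoot so the bookmark's up becomes world up, facing the camera's heading, at the pawn.
; FindAllBookmarks only counts tagged BP_Bookmark actors; its AllBookmarks assignment is disconnected.
; RotateAroundPoint is an unused debug experiment.
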(event EventBeginPlay
  (bind _self self)
  (bind _defaultsceneroot (Variables|Default|GetDefaultSceneRoot _self))
  (Utilities|FlowControl|Delay 0.2)
  (CallFunction|FindAllBookmarks)
  (bind _asvrpawn (Utilities|Casting|CastToVRPawn (Game|Player|GetPlayerPawn 0)))
  (Variables|/Game/VRTemplate/Blueprints/VRPawn.VRPawn_C|SetBookmarkController _asvrpawn _self)
  (Transformation|SetWorldLocation _defaultsceneroot (Transformation|GetWorldLocation (Variables|/Game/VRTemplate/Blueprints/VRPawn.VRPawn_C|GetRightHand _asvrpawn)) false true)
  (Transformation|SetWorldRotation _defaultsceneroot (Transformation|GetWorldRotation (Variables|/Game/VRTemplate/Blueprints/VRPawn.VRPawn_C|GetRightHand _asvrpawn)) false false)
  (Transformation|AttachComponentToComponent (Variables|/Game/VRTemplate/Blueprints/VRPawn.VRPawn_C|GetRightHand _asvrpawn) "None" "KeepWorld" "KeepWorld" "KeepWorld" true))

(fn ConstructionScript)

(fn FindAllBookmarks
  (bind _outactors (Actor|GetAllActorsOfClasswithTag "/Game/ARCH1510/Locomotion/BP_Bookmark.BP_Bookmark_C" "Bookmark"))
  (Variables|Default|SetNumberOfBookmarks (Utilities|Array|Length _outactors)))

(fn MoveNext
  (if (< (Variables|Default|GetCurrentBookmark) (Variables|Default|GetNumberOfBookmarks))
    (Math|Integer|IncrementInt (Variables|Default|GetCurrentBookmark)
      (:%20%20
        (CallFunction|TeleporttoBookmark)
        (CallFunction|UpdateName)))))

(fn MovePrevious
  (if (> (Variables|Default|GetCurrentBookmark) 1)
    (Math|Integer|DecrementInt (Variables|Default|GetCurrentBookmark)
      (:%20%20
        (CallFunction|TeleporttoBookmark)
        (CallFunction|UpdateName)))))

(fn TeleporttoBookmark
  (bind _allbookmarks (Variables|Default|GetAllBookmarks))
  (bind _currentbookmark (Variables|Default|GetCurrentBookmark))
  (bind _returnvalue (- _currentbookmark 1))
  (bind _output (Utilities|Array|Get(acopy) _allbookmarks _returnvalue))
  (bind _returnvalue_2 (Transformation|GetActorTransform _output))
  (if (Variables|Default|GetChangeGravity)
    (if (Utilities|IsValid (Variables|Default|GetWorldModelRoot))
      (CallFunction|Rotate))
    (else
      (Transformation|Teleport (Game|Player|GetPlayerPawn 0) (.location _returnvalue_2) (Math|Rotator|MakeRotator 0.0 0.0 (.yaw (.rotation _returnvalue_2)))))))

(fn RotateAroundPoint
  (bind _returnvalue (Math|Vector|VectorZero))
  (bind _allbookmarks (Variables|Default|GetAllBookmarks))
  (bind _test (Variables|Default|GetTest))
  (bind _currentbookmark (Variables|Default|GetCurrentBookmark))
  (bind _worldmodelroot (Variables|Default|GetWorldModelRoot))
  (bind _returnvalue_2 (- _currentbookmark 1))
  (bind _output (Utilities|Array|Get(acopy) _allbookmarks _returnvalue_2))
  (bind _arrow (Variables|/Game/ARCH1510/Locomotion/BP_Bookmark.BP_Bookmark_C|GetArrow _output))
  (bind _returnvalue_3 (Math|Vector|GetUpVector _arrow))
  (bind _returnvalue_4 (Math|Rotator|FindLookatRotation _returnvalue _returnvalue_3))
  (bind _returnvalue_5 (* _returnvalue_3 5e+02))
  (bind (_roll _pitch _yaw) (Math|Rotator|BreakRotator _returnvalue_4))
  (bind _returnvalue_6 (+ _pitch -9e+01))
  (bind _returnvalue_7 (Math|Rotator|MakeRotator _roll _returnvalue_6 _yaw))
  (bind _returnvalue_8 (Class|KismetMathLibrary|NegateRotator _returnvalue_7))
  (bind _output_get (LocalVariables|SetOriginalTransform (Transformation|GetActorTransform _worldmodelroot)))
  (Transformation|SetActorLocation _worldmodelroot "0, 0, 0" false true)
  (Transformation|SetActorRotation _test _returnvalue_8)
  (Class|Actor|AddActorWorldRotation _test _returnvalue_8)
  (Rendering|Debug|DrawDebugLine _returnvalue _returnvalue_5 "(R=1.000000,G=0.000000,B=0.017873,A=1.000000)" 5.0 5.0)
  (Rendering|Debug|DrawDebugLine _returnvalue (Math|Vector|RotateVector _returnvalue_5 _returnvalue_8) "(R=0.997933,G=0.000000,B=1.000000,A=1.000000)" 5.0 5.0))

(fn Rotate
  (bind _returnvalue (Math|Vector|VectorUp))
  (bind _returnvalue_2 (Game|GetPlayerCameraManager 0))
  (bind _worldmodelroot (Variables|Default|GetWorldModelRoot))
  (bind _allbookmarks (Variables|Default|GetAllBookmarks))
  (bind _currentbookmark (Variables|Default|GetCurrentBookmark))
  (bind _returnvalue_3 (Transformation|GetActorForwardVector _returnvalue_2))
  (bind _returnvalue_4 (- _currentbookmark 1))
  (bind _returnvalue_5 (Math|Vector|ProjectVectorontoPlane _returnvalue_3 _returnvalue))
  (bind _output (Utilities|Array|Get(acopy) _allbookmarks _returnvalue_4))
  (bind _returnvalue_6 (Math|Vector|Normalize _returnvalue_5))
  (bind _arrow (Variables|/Game/ARCH1510/Locomotion/BP_Bookmark.BP_Bookmark_C|GetArrow _output))
  (bind _returnvalue_7 (Math|Vector|GetForwardVector _arrow))
  (bind (_x _y) (Math|Vector|BreakVector _returnvalue_6))
  (bind (_x_2 _y_2) (Math|Vector|BreakVector _returnvalue_7))
  (Transformation|SetActorLocation _worldmodelroot "0, 0, 0" false true)
  (Class|Actor|AddActorWorldRotation _worldmodelroot (Class|KismetMathLibrary|NegateRotator (Math|Rotator|MakeRotfromXZ _returnvalue_7 (Transformation|GetActorUpVector _output))))
  (Class|Actor|AddActorWorldRotation _worldmodelroot (Math|Vector|RotatorfromAxisandAngle (Math|Vector|VectorUp) (- (Class|KismetMathLibrary|DegAtan2 _x_2 _y_2) (Class|KismetMathLibrary|DegAtan2 _x _y))))
  (Transformation|AddActorWorldOffset _worldmodelroot (- (Transformation|GetActorLocation (Game|Player|GetPlayerPawn 0)) (Transformation|GetActorLocation _output)) false true))

(fn UpdateName
  (bind _output_get (Variables|Default|SetCurrentLocationName (Variables|/Game/ARCH1510/Locomotion/BP_Bookmark.BP_Bookmark_C|GetBookmarkName (Utilities|Array|Get(acopy) (Variables|Default|GetAllBookmarks) (- (Variables|Default|GetCurrentBookmark) 1)))))
  (Rendering|Components|TextRender|SetText (Variables|Default|GetTextRender) _output_get))